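; BP_Han is a Blueprint that puts the player aim point widget on screen at BeginPlay.
; Tick casts a player state to ProjectPlayerState every frame, but no live logic uses the result.
; Disconnected test nodes, which never run, would apply the GE_ABlaze gameplay effect to its own Ability System Component and print that player state's health.
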(event EventBeginPlay
  (bind _returnvalue (UserInterface|CreateWidget "/Game/UI/WBP_PlayerAimPoint.WBP_PlayerAimPoint_C"))
  (UserInterface|Viewport|AddtoViewport _returnvalue 0))

(event Collision|EventActorBeginOverlap
  (params (OtherActor :type Actor%20Object%20Reference)))

(event EventTick
  (params (DeltaSeconds :type Float%20%28single-precision%29))
  (bind _asproject_player_state (Utilities|Casting|CastToProjectPlayerState (Game|GetPlayerState 3))))

(fn ConstructionScript)