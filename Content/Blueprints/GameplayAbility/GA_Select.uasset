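; GA_Select is a gameplay ability that shows a selection wheel for the player's equipped ability data while the input is held.
; On activation it reads the selected ability data from the character's EquipComponent and creates WBP_SelectWidget with its option count, text and the previous SelectNumber.
; Releasing the input ends the ability, which saves the widget's last angle into SelectNumber and removes it.
; Without valid ability data it ends immediately.
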(event Ability|EventOnEndAbility
  (params (bWasCancelled :type Boolean))
  (bind _selectwidget (Variables|Default|GetSelectWidget))
  (Utilities|IsValid _selectwidget
    (:Is%20Valid
      (bind _lastangle (Default|GetLastAngle _selectwidget))
      (Variables|/Script/SkySeoul.SkySeoulCharacter|SetSelectNumber (Variables|Default|GetPlayerCharacter) _lastangle)
      (Widget|RemovefromParent _selectwidget))))

(event Ability|EventActivateAbility
  (bind _assky_seoul_character (Utilities|Casting|CastToSkySeoulCharacter (Class|CharacterGameplayAbility|GetCharacterfromActorInfo)))
  (Variables|Default|SetPlayerCharacter _assky_seoul_character)
  (bind _returnvalue (Class|EquipmentComponent|GetSelectedAbilityData (Variables|/Script/SkySeoul.SkySeoulCharacter|GetEquipComponent _assky_seoul_character)))
  (Utilities|IsValid _returnvalue
    (:Is%20Valid
      (bind _returnvalue_2 (Class|AbilitySetData|GetAbilityCount _returnvalue))
      (bind _returnvalue_3 (Class|AbilitySetData|SelectAbilityText _returnvalue))
      (bind _returnvalue_4 (UserInterface|CreateWidget "/Game/UI/SelectWidget/WBP_SelectWidget.WBP_SelectWidget_C" 0 _returnvalue_2 (Variables|/Script/SkySeoul.SkySeoulCharacter|GetSelectNumber (Variables|Default|GetPlayerCharacter)) _returnvalue_3))
      (bind _output_get (Variables|Default|SetSelectWidget _returnvalue_4))
      (UserInterface|Viewport|AddtoViewport _output_get 0)
      (Ability|Tasks|WaitInputRelease false
        (:OnRelease
          (Ability|EndAbility))))
    (:Is%20Not%20Valid
      (Ability|EndAbility))))