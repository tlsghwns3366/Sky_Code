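; GA_PeanutMessage is a gameplay ability that shows a Peanut widget's messages one at a time.
; It takes the WBP_Peanut from the triggering event's OptionalObject and fills its MessageBox with a new WBP_PeanutMessage for the current entry.
; Each Ability.Player.Peanut.HideMessage gameplay event advances the index and loops back.
; After the last entry it resets the index, ends the ability and plays HideWidget before removing the widget.
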(event Ability|EventActivateAbilityFromEvent
  (params (EventData :type Gameplay%20Event%20Data%20Structure%20%28by%20ref%29))
  (Ability|CommitAbility)
  (bind _aswbp_peanut (Utilities|Casting|CastToWBP_Peanut (.OptionalObject (Utilities|Struct|BreakGameplayEventData EventData))))
  (Variables|Default|SetPeanutWidget _aswbp_peanut)
  (if (== (Utilities|Array|Length (Variables|/Game/UI/MessageWidget/WBP_Peanut.WBP_Peanut_C|GetPeanutMessage _aswbp_peanut)) (Variables|Default|GetCurrentInt)) :!label _label
    (Variables|Default|SetCurrentInt 0)
    (Ability|EndAbility)
    (Components|Animation|PlayAnimation (Variables|Default|GetPeanutWidget) (Variables|/Game/UI/MessageWidget/WBP_Peanut.WBP_Peanut_C|GetHideWidget (Variables|Default|GetPeanutWidget)) 0.0
      (:Finished
        (Widget|RemovefromParent (Variables|Default|GetPeanutWidget))))
    (else
      (Widget|Panel|ClearChildren (Variables|/Game/UI/MessageWidget/WBP_Peanut.WBP_Peanut_C|GetMessageBox _aswbp_peanut))
      (bind _returnvalue (UserInterface|CreateWidget "/Game/UI/MessageWidget/WBP_PeanutMessage.WBP_PeanutMessage_C" 0 (Utilities|Array|Get(acopy) (Variables|/Game/UI/MessageWidget/WBP_Peanut.WBP_Peanut_C|GetPeanutMessage (Variables|Default|GetPeanutWidget)) (Variables|Default|GetCurrentInt))))
      (Widget|Panel|AddChild (Variables|/Game/UI/MessageWidget/WBP_Peanut.WBP_Peanut_C|GetMessageBox (Variables|Default|GetPeanutWidget)) _returnvalue)
      (Ability|Tasks|WaitGameplayEvent "(TagName=\"Ability.Player.Peanut.HideMessage\")" 0 true
        (:EventReceived
          (Variables|Default|SetCurrentInt (+ (Variables|Default|GetCurrentInt) 1))
          (goto _label))))))