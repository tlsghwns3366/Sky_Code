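; GA_QuickSlot6 is a quick slot gameplay ability that triggers use of the item held in the character's slot at QuickSlotNumber.
; On activation it commits, reads that slot from the SkySeoulCharacter's EquipComponent and, if valid, sets it as the selected item.
; It then sends a gameplay event with the item's UseAbilityTag, passing the character as instigator and the item as payload object, and ends.
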(event Ability|EventActivateAbility
  (Ability|CommitAbility)
  (bind _assky_seoul_character (Utilities|Casting|CastToSkySeoulCharacter (Class|CharacterGameplayAbility|GetCharacterfromActorInfo))
    (:then
      (bind _output_get (Variables|Default|SetEquip%20Component (Variables|/Script/SkySeoul.SkySeoulCharacter|GetEquipComponent _assky_seoul_character)))
      (Utilities|IsValid (Utilities|Array|Get(acopy) (Variables|/Script/SkySeoul.EquipmentComponent|GetQuickSlotItem _output_get) (Variables|Default|GetQuickSlotNumber))
        (:Is%20Valid
          (Class|EquipmentComponent|SetSelectItem (Variables|Default|GetEquip%20Component) (Utilities|Array|Get(acopy) (Variables|/Script/SkySeoul.EquipmentComponent|GetQuickSlotItem _output_get) (Variables|Default|GetQuickSlotNumber)))
          (Ability|SendGameplayEvent (Variables|/Script/SkySeoul.ItemObject|GetUseAbilityTag (Utilities|Array|Get(acopy) (Variables|/Script/SkySeoul.EquipmentComponent|GetQuickSlotItem _output_get) (Variables|Default|GetQuickSlotNumber))) (Utilities|Struct|MakeGameplayEventData (Variables|/Script/SkySeoul.ItemObject|GetUseAbilityTag (Utilities|Array|Get(acopy) (Variables|/Script/SkySeoul.EquipmentComponent|GetQuickSlotItem _output_get) (Variables|Default|GetQuickSlotNumber))) _assky_seoul_character 0 (Utilities|Array|Get(acopy) (Variables|/Script/SkySeoul.EquipmentComponent|GetQuickSlotItem _output_get) (Variables|Default|GetQuickSlotNumber))))
          (Ability|EndAbility))
        (:Is%20Not%20Valid
          (Ability|EndAbility))))
    (:CastFailed
      (Ability|EndAbility))))