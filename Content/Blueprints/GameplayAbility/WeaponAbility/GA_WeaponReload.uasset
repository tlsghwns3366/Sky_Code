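; Gameplay ability that reloads the gun currently selected in a SkySeoulCharacter's equip component.
; On event activation it waits for the reload time, then calls SetCurrentMagazine on the gun with the character's inventory component and ends.
; It ends immediately if the character or selected gun cast fails.
; Any ending sends a ReloadFinish gameplay event to the character.
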(event Ability|EventOnEndAbility
  (params (bWasCancelled :type Boolean))
  (Ability|SendGameplayEventtoActor (Class|CharacterGameplayAbility|GetCharacterfromActorInfo) "(TagName=\"Ability.Player.Weapon.ReloadFinish\")"))

(event Ability|EventActivateAbilityFromEvent
  (params (EventData :type Gameplay%20Event%20Data%20Structure%20%28by%20ref%29))
  (bind _assky_seoul_character (Utilities|Casting|CastToSkySeoulCharacter (Class|CharacterGameplayAbility|GetCharacterfromActorInfo))
    (:then
      (bind _asgun_weapon_object (Utilities|Casting|CastToGunWeaponObject (Class|EquipmentComponent|GetSelectedItem (Variables|/Script/SkySeoul.SkySeoulCharacter|GetEquipComponent _assky_seoul_character)))
        (:then
          (Ability|Tasks|WaitDelay (Variables|Default|GetReloadTime)
            (:OnFinish
              (Class|GunWeaponObject|SetCurrentMagazine _asgun_weapon_object (Variables|/Script/SkySeoul.SkySeoulCharacter|GetInventoryComponent _assky_seoul_character))
              (Ability|EndAbility))))
        (:CastFailed
          (Ability|EndAbility))))
    (:CastFailed
      (Ability|EndAbility))))