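; Default weapon-fire Gameplay Ability that fires a shot and handles hits on targets.
; A successful commit pays the cost, calls OnFire and starts a fire-delay timer, with FireComplete ending the ability.
; A failed commit sends a Reload gameplay event to the character and ends upon receiving ReloadFinish.
; TargetHit plays a gameplay cue from the hit result and applies the damage GameplayEffect to the target.
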(event Custom|FireComplete
  (Ability|EndAbility))

(event EventTargetHit
  (params (TargetData :type Gameplay%20Ability%20Target%20Data%20Handle%20Structure%20%28by%20ref%29))
  (Class|GameplayAbility|ExecuteGameplayCuewithParams (Variables|Default|GetGameplay%20Cue%20Tag) (GameplayCue|MakeGameplayCueParametersfromHitResult (Ability|TargetData|GetHitResultfromTargetData TargetData)))
  (GameplayEffects|ApplyGameplayEffectToTarget TargetData (Variables|Default|GetGE_Damage) (Variables|Default|GetGameplay%20Effect%20Level) 1))

(event Ability|EventCommitExecute
  (Ability|CommitAbilityCost false)
  (Class|WeaponGameplayAbility|OnFire)
  (Utilities|Time|SetTimerbyEvent (EventDispatchers|CreateEvent :!event Custom|FireComplete) (Variables|Default|GetFireDelayTimeSecs)))

(event Ability|EventActivateAbility
  (bind _returnvalue (Ability|CommitAbility))
  (if (not _returnvalue)
    (Ability|Tasks|WaitGameplayEvent "(TagName=\"Ability.Player.Weapon.ReloadFinish\")" 0
      (:then
        (Ability|SendGameplayEventtoActor (Class|CharacterGameplayAbility|GetCharacterfromActorInfo) "(TagName=\"Ability.Player.Weapon.Reload\")"))
      (:EventReceived
        (Ability|EndAbility)))))