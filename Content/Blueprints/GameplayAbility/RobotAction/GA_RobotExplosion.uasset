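; Gameplay Ability that detonates the player's currently selected robot.
; On activation it commits, then looks up the robot at SelectRobotNumber in the SkySeoulCharacter's RobotArray.
; A valid robot is removed from the character through RemoveRobot, then told to run its own RobotExplosion.
; The ability ends immediately afterward, or without effect if the cast or validity check fails.
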(event Ability|EventActivateAbility
  (Ability|CommitAbility)
  (bind _assky_seoul_character (Utilities|Casting|CastToSkySeoulCharacter (Class|CharacterGameplayAbility|GetCharacterfromActorInfo))
    (:then
      (Utilities|IsValid (Utilities|Array|Get(acopy) (Variables|/Script/SkySeoul.SkySeoulCharacter|GetRobotArray _assky_seoul_character) (Variables|/Script/SkySeoul.SkySeoulCharacter|GetSelectRobotNumber _assky_seoul_character))
        (:Is%20Valid
          (Variables|Default|SetRobotCharacter (Utilities|Array|Get(acopy) (Variables|/Script/SkySeoul.SkySeoulCharacter|GetRobotArray _assky_seoul_character) (Variables|/Script/SkySeoul.SkySeoulCharacter|GetSelectRobotNumber _assky_seoul_character)))
          (Class|SkySeoulCharacter|RemoveRobot _assky_seoul_character (Variables|/Script/SkySeoul.SkySeoulCharacter|GetSelectRobotNumber _assky_seoul_character))
          (Class|RobotCharacter|RobotExplosion (Variables|Default|GetRobotCharacter))
          (Ability|EndAbility))
        (:Is%20Not%20Valid
          (Ability|EndAbility :!label _label))))
    (:CastFailed
      (goto _label))))