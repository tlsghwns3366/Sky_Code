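; GA_RobotIsFree is a gameplay ability that releases the player character's currently selected robot.
; On activation it commits, casts the avatar to SkySeoulCharacter and reads the RobotArray entry at SelectRobotNumber.
; A valid robot is cached, removed from the character via RemoveRobot, then told RobotIsFree.
; The ability ends immediately, including when the cast or validity check fails.
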(event Ability|EventActivateAbility
  (Ability|CommitAbility)
  (bind _assky_seoul_character (Utilities|Casting|CastToSkySeoulCharacter (Class|CharacterGameplayAbility|GetCharacterfromActorInfo))
    (:then
      (Utilities|IsValid (Utilities|Array|Get(acopy) (Variables|/Script/SkySeoul.SkySeoulCharacter|GetRobotArray _assky_seoul_character) (Variables|/Script/SkySeoul.SkySeoulCharacter|GetSelectRobotNumber _assky_seoul_character))
        (:Is%20Valid
          (bind _output_get (Variables|Default|SetRobotCharacter (Utilities|Array|Get(acopy) (Variables|/Script/SkySeoul.SkySeoulCharacter|GetRobotArray _assky_seoul_character) (Variables|/Script/SkySeoul.SkySeoulCharacter|GetSelectRobotNumber _assky_seoul_character))))
          (Class|SkySeoulCharacter|RemoveRobot _assky_seoul_character (Variables|/Script/SkySeoul.SkySeoulCharacter|GetSelectRobotNumber _assky_seoul_character))
          (Class|RobotCharacter|RobotIsFree _output_get)
          (Ability|EndAbility))
        (:Is%20Not%20Valid
          (Ability|EndAbility :!label _label))))
    (:CastFailed
      (goto _label))))