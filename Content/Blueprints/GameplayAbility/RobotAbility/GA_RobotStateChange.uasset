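; Gameplay ability that cycles the behavior state of the player's currently selected robot companion.
; On activation it commits, gets the SkySeoulCharacter and reads its RobotArray at SelectRobotNumber.
; The robot's state advances in a loop from Peace to Preemptive Attack to Under Attack and back through StateChange.
; The ability then ends, or ends immediately when the array is empty.
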(event Ability|EventActivateAbility
  (Ability|CommitAbility)
  (bind _assky_seoul_character (Utilities|Casting|CastToSkySeoulCharacter (Class|CharacterGameplayAbility|GetCharacterfromActorInfo)))
  (bind _output_get (Variables|Default|SetPlayerCharacter _assky_seoul_character))
  (if (Utilities|Array|IsEmpty (Variables|/Script/SkySeoul.SkySeoulCharacter|GetRobotArray _output_get))
    (Ability|EndAbility)
    (else
      (switch Utilities|FlowControl|Switch|SwitchonERobotState (Variables|/Script/SkySeoul.RobotCharacter|GetRobotState (Utilities|Array|Get(acopy) (Variables|/Script/SkySeoul.SkySeoulCharacter|GetRobotArray _output_get) (Variables|/Script/SkySeoul.SkySeoulCharacter|GetSelectRobotNumber _output_get)))
        (:E_Peace
          (Class|RobotCharacter|StateChange (Utilities|Array|Get(acopy) (Variables|/Script/SkySeoul.SkySeoulCharacter|GetRobotArray _output_get) (Variables|/Script/SkySeoul.SkySeoulCharacter|GetSelectRobotNumber _output_get)) "E_PreemptiveAttack"))
        (:E_PreemptiveAttack
          (Class|RobotCharacter|StateChange (Utilities|Array|Get(acopy) (Variables|/Script/SkySeoul.SkySeoulCharacter|GetRobotArray _output_get) (Variables|/Script/SkySeoul.SkySeoulCharacter|GetSelectRobotNumber _output_get)) "E_UnderAttack"))
        (:E_UnderAttack
          (Class|RobotCharacter|StateChange (Utilities|Array|Get(acopy) (Variables|/Script/SkySeoul.SkySeoulCharacter|GetRobotArray _output_get) (Variables|/Script/SkySeoul.SkySeoulCharacter|GetSelectRobotNumber _output_get)) "E_Peace")))
      (Ability|EndAbility))))