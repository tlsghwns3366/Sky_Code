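; Gameplay ability that orders the player's currently selected robot to move to a target location.
; On activation it commits, casts the avatar to SkySeoulCharacter and picks the robot at SelectRobotNumber in its RobotArray.
; If that robot is valid, it sets the MoveLocation action state and calls MoveAction with the character's stored RobotLocation.
; The ability ends immediately on every path, leaving the movement itself to the robot.
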(event Ability|EventActivateAbility
  (Ability|CommitAbility)
  (bind _assky_seoul_character (Utilities|Casting|CastToSkySeoulCharacter (Class|CharacterGameplayAbility|GetCharacterfromActorInfo))
    (:then
      (Utilities|IsValid (Utilities|Array|Get(acopy) (Variables|/Script/SkySeoul.SkySeoulCharacter|GetRobotArray _assky_seoul_character) (Variables|/Script/SkySeoul.SkySeoulCharacter|GetSelectRobotNumber _assky_seoul_character))
        (:Is%20Valid
          (Class|RobotCharacter|SetRobotActionState (Utilities|Array|Get(acopy) (Variables|/Script/SkySeoul.SkySeoulCharacter|GetRobotArray _assky_seoul_character) (Variables|/Script/SkySeoul.SkySeoulCharacter|GetSelectRobotNumber _assky_seoul_character)) "E_MoveLocation")
          (Class|RobotCharacter|MoveAction (Utilities|Array|Get(acopy) (Variables|/Script/SkySeoul.SkySeoulCharacter|GetRobotArray _assky_seoul_character) (Variables|/Script/SkySeoul.SkySeoulCharacter|GetSelectRobotNumber _assky_seoul_character)) (Variables|/Script/SkySeoul.SkySeoulCharacter|GetRobotLocation _assky_seoul_character))
          (Ability|EndAbility))
        (:Is%20Not%20Valid
          (Ability|EndAbility :!label _label))))
    (:CastFailed
      (goto _label))))