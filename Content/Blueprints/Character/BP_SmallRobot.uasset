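; BP_SmallRobot is a robot character Blueprint that sets up on-robot UI for interaction, hacking and player selection.
; On BeginPlay it creates the interaction, hacking ("E" prompt) and select widgets and assigns them to their widget components.
; Bound update events push HackingPercent into the hacking widget's material scalar and IsSelect into the select widget.
; Tick and overlap events are empty, and a health-printing chain is left unconnected.
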(event Custom|SelectUpdate
  (Default|SetSelect (Variables|Default|GetSelectWidgetBlueprint) (Variables|Default|GetIsSelect)))

(event Custom|커스텀이벤트
  (Default|SetMaterialScalar (Variables|Default|GetButtonWidget) (Variables|Default|GetHackingPercent)))

(event EventBeginPlay
  (bind _returnvalue (UserInterface|CreateWidget "/Game/UI/PlayerHud/WBP_InteractionWidget.WBP_InteractionWidget_C"))
  (UserInterface|SetWidget (Variables|Default|GetInteractionWidgetComponent) _returnvalue)
  (bind _returnvalue_2 (UserInterface|CreateWidget "/Game/UI/PlayerHud/WBP_HackingUI.WBP_HackingUI_C" 0 "E"))
  (bind _output_get (Variables|Default|SetButtonWidget _returnvalue_2))
  (UserInterface|SetWidget (Variables|Default|GetButtonWidgetComponent) _output_get)
  (EventDispatchers|BindEventtoHackingUpdate (delegate Custom|커스텀이벤트))
  (bind _returnvalue_3 (UserInterface|CreateWidget "/Game/UI/Robot/WBP_RobotSelect.WBP_RobotSelect_C"))
  (bind _output_get_2 (Variables|Default|SetSelectWidgetBlueprint _returnvalue_3))
  (UserInterface|SetWidget (Variables|Default|GetSelectWidget) _output_get_2)
  (EventDispatchers|BindEventtoPlayerSelectUpdate (delegate Custom|SelectUpdate)))

(event Collision|EventActorBeginOverlap
  (params (OtherActor :type Actor%20Object%20Reference)))

(event EventTick
  (params (DeltaSeconds :type Float%20%28single-precision%29)))

(fn ConstructionScript)