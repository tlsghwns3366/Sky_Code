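; BP_Han is a player character Blueprint that sets up HUD widgets and handles weapon-switch input.
; BeginPlay adds the aim point and robot list widgets, passing the character to the latter.
; The IA_MouseWheel action cycles weapons up or down through EquipComponent by scroll direction.
; Releasing H enables mesh physics and J shows a WBP_Peanut message, while disconnected nodes hold health, weapon and gameplay-effect snippets that never run.
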(event Input|EnhancedActionEvents|EnhancedInputActionIA_MouseWheel
  (params (ActionValue :type Float%20%28double-precision%29) (ElapsedSeconds :type Float%20%28double-precision%29) (TriggeredSeconds :type Float%20%28double-precision%29) (InputAction :type Input%20Action%20Object%20Reference :default "/Game/Input/Actions/IA_MouseWheel.IA_MouseWheel"))
  (bind _equipcomponent (Variables|Default|GetEquipComponent))
  (if (> ActionValue 0.0)
    (Class|EquipmentComponent|WeaponChangeUp _equipcomponent)
    (else
      (Class|EquipmentComponent|WeaponChangeDown _equipcomponent))))

(event EventBeginPlay
  (bind _returnvalue (UserInterface|CreateWidget "/Game/UI/PlayerHud/WBP_PlayerAimPoint.WBP_PlayerAimPoint_C"))
  (UserInterface|Viewport|AddtoViewport _returnvalue 0)
  (bind _returnvalue_2 (UserInterface|CreateWidget "/Game/UI/Robot/WBP_RobotList.WBP_RobotList_C" 0 self))
  (UserInterface|Viewport|AddtoViewport _returnvalue_2 0))

(event Collision|EventActorBeginOverlap
  (params (OtherActor :type Actor%20Object%20Reference)))

(event EventTick
  (params (DeltaSeconds :type Float%20%28single-precision%29)))

(event Input|KeyboardEvents|H
  (params (Key :type Key%20Structure))
  (:Released
    (Physics|SetSimulatePhysics (Variables|Character|GetMesh) true)))

(event Input|KeyboardEvents|J
  (params (Key :type Key%20Structure))
  (:Released
    (bind _returnvalue (UserInterface|CreateWidget "/Game/UI/MessageWidget/WBP_Peanut.WBP_Peanut_C" 0 (Variables|Default|GetTempString)))
    (UserInterface|Viewport|AddtoViewport _returnvalue 0)))

(fn ConstructionScript)